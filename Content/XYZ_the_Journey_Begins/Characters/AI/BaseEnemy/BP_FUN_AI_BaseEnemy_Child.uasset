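; Child Blueprint of the base AI enemy, a "FUN" variant that adds a dancing behavior.
; The FUN_Dancing event plays a dancing montage on the mesh.
; OnDeath unpossesses the controller, stops the current weapon firing and plays a death montage if the mesh is valid.
; The Box overlap handler is empty, and the construction script only calls the parent's.
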(event OnComponentBeginOverlap(Box)
  (params (OverlappedComponent :type Primitive%20Component%20Object%20Reference) (OtherActor :type Actor%20Object%20Reference) (OtherComp :type Primitive%20Component%20Object%20Reference) (OtherBodyIndex :type Integer) (bFromSweep :type Boolean) (SweepResult :type Hit%20Result%20Structure%20%28by%20ref%29)))

(event Custom|FUN_Dancing
  (Animation|Montage|PlayMontage (Variables|Character|GetMesh) "/Game/XYZ_the_Journey_Begins/Characters/AI/BaseEnemy/Animations/FUN/Dancing_Montage.Dancing_Montage"))

(event EventBeginPlay
  (|CallParentFunction) ; This node is disabled and will not be called.\nDrag off pins to build functionality.
)

(event EventTick
  (params (DeltaSeconds :type Float%20%28single-precision%29)))

(event Collision|EventActorBeginOverlap
  (params (OtherActor :type Actor%20Object%20Reference)))

(event EventOnDeath
  (bind _mesh (Variables|Character|GetMesh))
  (Pawn|UnPossess (Pawn|GetController))
  (Default|StopShoot (Variables|Default|GetCurrentWeapon))
  (Utilities|IsValid _mesh
    (:Is%20Valid
      (Animation|Montage|PlayMontage _mesh (Variables|Default|GetDeathMontage)))))

(fn ConstructionScript
  (|CallParentFunction))
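; BP_PlayerController is a player controller that opens the pause menu when the GamePause input is pressed.
; If not already paused, it creates and shows WBP_Pause_Menu, enables the mouse cursor with Game and UI input focused on the widget, and pauses the game.
; Its unpause logic is disconnected and marked deprecated, with a note pointing to the widget's logic instead.
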(event Input|ActionEvents|InputActionGamePause
  (params (Key :type Key%20Structure :default "None"))
  (:Pressed
    (if (not (Variables|Default|GetbIsGamePaused))
      (Variables|Default|SetbIsGamePaused true)
      (bind _returnvalue (UserInterface|CreateWidget "/Game/XYZ_the_Journey_Begins/Widgets/WBP_Pause_Menu.WBP_Pause_Menu_C"))
      (UserInterface|Viewport|AddtoViewport _returnvalue 0)
      (Variables|Default|SetbShowMouseCursor true)
      (Input|SetInputModeGameandUI self _returnvalue "DoNotLock" true)
      (Game|SetGamePaused true)
      (Development|PrintString "GAME PAUSED"))))

(fn ConstructionScript)
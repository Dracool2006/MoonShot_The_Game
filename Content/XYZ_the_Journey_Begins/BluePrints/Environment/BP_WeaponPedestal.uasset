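; Weapon pedestal pickup that displays a Pistol or Shotgun and grants it to the player on touch.
; BeginPlay sets the skeletal mesh from the PedestalWeapon value.
; When BP_PlayerCharacter overlaps the box, it passes that value to the character's BeginPlaySpawnWeaponsEvent.
; It then destroys the mesh and trigger components, leaving the actor in place, and plays the pickup sound.
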(event OnComponentBeginOverlap(BoxCollision)
  (params (OverlappedComponent :type Primitive%20Component%20Object%20Reference) (OtherActor :type Actor%20Object%20Reference) (OtherComp :type Primitive%20Component%20Object%20Reference) (OtherBodyIndex :type Integer) (bFromSweep :type Boolean) (SweepResult :type Hit%20Result%20Structure%20%28by%20ref%29))
  (bind _asbp_player_character (Utilities|Casting|CastToBP_PlayerCharacter OtherActor))
  (Default|BeginPlaySpawnWeaponsEvent _asbp_player_character (Variables|Default|GetPedestalWeapon))
  (Components|DestroyComponent (Variables|Default|GetSkeletalMesh))
  (Audio|Components|Audio|Play (Variables|Default|GetSound_PickUpWeapon) 0.0))

(event EventBeginPlay
  (switch Utilities|FlowControl|Switch|SwitchonENUM_WeaponTypes (Variables|Default|GetPedestalWeapon)
    (:NewEnumerator0
      (Class|SkinnedMeshComponent|SetSkeletalMesh (Variables|Default|GetSkeletalMesh) "/Game/XYZ_the_Journey_Begins/Weapons/Pistol/SK_Pistol.SK_Pistol" false))
    (:NewEnumerator1
      (Class|SkinnedMeshComponent|SetSkeletalMesh (Variables|Default|GetSkeletalMesh) "/Game/XYZ_the_Journey_Begins/Weapons/Shotgun/SK_Shotgun.SK_Shotgun" false))))

(fn ConstructionScript)
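; BP_BasePlayerWeapon is the base Blueprint for player weapons, aligning the firing barrel with the player's camera aim.
; Its UpdateBarrelLocation override calls the parent, then casts and caches the owner as BP_PlayerCharacter.
; It moves EBBarrel to where the follow camera's forward line crosses the muzzle's facing plane and copies the camera's rotation, keeping the barrel on the view axis at muzzle depth.
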(event EventUpdateBarrelLocation
  (bind _muzzlelocation (Variables|Default|GetMuzzleLocation))
  (|CallParentFunction)
  (bind _asbp_player_character (Utilities|Casting|CastToBP_PlayerCharacter (Variables|Default|GetWeaponOwner)))
  (Variables|Default|SetPlayerWeaponOwner _asbp_player_character)
  (Transformation|SetWorldLocation (Variables|Default|GetEBBarrel) (.Intersection (Class|KismetMathLibrary|LinePlaneIntersectionOriginNormal (Transformation|GetWorldLocation (Variables|/Game/XYZ_the_Journey_Begins/Characters/Player/BP_PlayerCharacter.BP_PlayerCharacter_C|GetFollowCamera (Variables|Default|GetPlayerWeaponOwner))) (+ (Transformation|GetWorldLocation (Variables|/Game/XYZ_the_Journey_Begins/Characters/Player/BP_PlayerCharacter.BP_PlayerCharacter_C|GetFollowCamera (Variables|Default|GetPlayerWeaponOwner))) (* (Math|Vector|GetForwardVector (Variables|/Game/XYZ_the_Journey_Begins/Characters/Player/BP_PlayerCharacter.BP_PlayerCharacter_C|GetFollowCamera (Variables|Default|GetPlayerWeaponOwner))) 1e+03)) (Transformation|GetWorldLocation _muzzlelocation) (Math|Vector|GetForwardVector _muzzlelocation))) false false)
  (Transformation|SetWorldRotation (Variables|Default|GetEBBarrel) (Transformation|GetWorldRotation (Variables|/Game/XYZ_the_Journey_Begins/Characters/Player/BP_PlayerCharacter.BP_PlayerCharacter_C|GetFollowCamera (Variables|Default|GetPlayerWeaponOwner))) false false))

(fn ConstructionScript
  (|CallParentFunction))
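; Base weapon Blueprint that wraps an EBBarrel ballistics component for shooting, magazine and reserve ammo, and reloading.
; Shots trigger muzzle flash plus weapon and character montages, while an empty UpdateBarrelLocation hook is called during firing.
; StartReload blocks shooting and plays animation and sound; a separate EndReload moves reserve ammo into the barrel.
; Gravity changes reload the barrel with matching shotgun bullets and set its fire rate.
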(event Custom|StartShoot
  ;[1 1 1] Start and Stop Shoot Events
  (if (not (Variables|/Script/EasyBallistics.EBBarrel|GetShootingBlocked (Variables|Default|GetEBBarrel)))
    (Variables|Default|SetbIsShooting true)
    (CallFunction|UpdateBarrelLocation)
    (Class|EBBarrel|Shoot (Variables|Default|GetEBBarrel) true)))

(event Custom|StopShoot
  ;[1 1 1] Start and Stop Shoot Events
  (Variables|Default|SetbIsShooting false)
  (Class|EBBarrel|Shoot (Variables|Default|GetEBBarrel) false)
  (Transformation|SetWorldTransform (Variables|Default|GetEBBarrel) (Transformation|GetWorldTransform (Variables|Default|GetMuzzleFlash)) false false))

(event Custom|OnShotFired
  (Components|Activation|Activate (Variables|Default|GetMuzzleFlash) true)
  (Animation|Montage|PlayMontage (Variables|Default|GetWeapon_SkeletalMesh) (Variables|Default|GetWeaponShotMontage)
    (:then
      (Animation|Montage|PlayMontage (Variables|/Script/Engine.Character|GetMesh (Variables|Default|GetWeaponOwner)) (Variables|Default|GetCharacterShotMontage)))))

(event Custom|Reloading
  (Variables|Default|SetCurrentRemainingAmmo (Variables|Default|GetMaxRemainingAmmo)))

(event Custom|Weapon%20Change%20Gravity
  (params (GravityType :type ENUM_GravityDoorType%20Enum :default "NewEnumerator0"))
  (bind _ebbarrel (Variables|Default|GetEBBarrel))
  (bind _ebbarrel_2 (Variables|Default|GetEBBarrel))
  (bind _ebbarrel_3 (Variables|Default|GetEBBarrel))
  (bind _ebbarrel_4 (Variables|Default|GetEBBarrel))
  (switch Utilities|FlowControl|Switch|SwitchonENUM_GravityDoorType GravityType
    (:NewEnumerator0
      (Class|EBBarrel|SetAmmo (Variables|Default|GetEBBarrel) 8 true false false (Variables|Default|GetHighGravityShotgunBullets))
      (Variables|/Script/EasyBallistics.EBBarrel|SetFireRateMin _ebbarrel 1.0)
      (Variables|/Script/EasyBallistics.EBBarrel|SetFireRateMax _ebbarrel 1.0))
    (:NewEnumerator1
      (Class|EBBarrel|SetAmmo (Variables|Default|GetEBBarrel) 8 true false false (Variables|Default|GetMediumGravityShotgunBullets))
      (Variables|/Script/EasyBallistics.EBBarrel|SetFireRateMin _ebbarrel_3 1.0)
      (Variables|/Script/EasyBallistics.EBBarrel|SetFireRateMax _ebbarrel_3 1.0))
    (:NewEnumerator2
      (Class|EBBarrel|SetAmmo (Variables|Default|GetEBBarrel) 8 true false false (Variables|Default|GetLowGravityShotgunBullets))
      (Variables|/Script/EasyBallistics.EBBarrel|SetFireRateMin _ebbarrel_4 8.0)
      (Variables|/Script/EasyBallistics.EBBarrel|SetFireRateMax _ebbarrel_4 8.0))
    (:NewEnumerator3
      (Class|EBBarrel|SetAmmo (Variables|Default|GetEBBarrel) 8 true false false (Variables|Default|GetFUNGravityShotgunBullets))
      (Variables|/Script/EasyBallistics.EBBarrel|SetFireRateMin _ebbarrel_2 1.0)
      (Variables|/Script/EasyBallistics.EBBarrel|SetFireRateMax _ebbarrel_2 1.0))))

(event EventBeginPlay
  (CallFunction|Reloading)
  (EventDispatchers|BindEventtoShotFired (Variables|Default|GetEBBarrel) (delegate Custom|OnShotFired)))

(event EventTick
  (params (DeltaSeconds :type Float%20%28single-precision%29))
  (Utilities|FlowControl|Sequence
    (:then_0
      (CallFunction|DebugDraw false))
    (:then_1
      (if (Variables|Default|GetbIsShooting)
        (CallFunction|UpdateBarrelLocation)))
    (:then_2
      (|DebugAmmoGraph))))

(fn ConstructionScript)

(fn UpdateBarrelLocation
  ;[1 1 1] Function Only For Player
)

(fn DebugDraw
  (params (bISEnableDebug :type Boolean))
  (bind _muzzlelocation (Variables|Default|GetMuzzleLocation))
  (bind _ebbarrel (Variables|Default|GetEBBarrel))
  (bind _returnvalue (Transformation|GetWorldLocation _muzzlelocation))
  (bind _returnvalue_2 (Transformation|GetWorldLocation _ebbarrel))
  (if bISEnableDebug
    (Rendering|Debug|DrawDebugLine _returnvalue _returnvalue_2 "(R=0.930111,G=0.829365,B=0.422403,A=1.000000)" 0.0 5.0)
    (Rendering|Debug|DrawDebugSphere _returnvalue 2e+01 12 "(R=0.741148,G=1.000000,B=0.663750,A=1.000000)" 0.0)
    (Rendering|Debug|DrawDebugSphere _returnvalue_2 1e+01 12 "(R=0.103198,G=0.114191,B=1.000000,A=1.000000)" 0.0)))

(fn GetRequiredAmmo
  (bind _magazinesize (Variables|Default|GetMagazineSize))
  (Variables|Default|SetRequiredAmmoCount (Math|Integer|Clamp(Integer) (- _magazinesize (Class|EBBarrel|GetAmmoCount (Variables|Default|GetEBBarrel) true)) 0 _magazinesize))
  (return))

(fn StartReload
  (if (Variables|Default|GetbIsReloading)
    (Development|PrintString "isReloading")
    (elif (> (Variables|Default|GetCurrentRemainingAmmo) 0)
      (CallFunction|GetRequiredAmmo)
      (if (== (Variables|Default|GetRequiredAmmoCount) 0)
        (Development|PrintString "AmmoAlreadyIsFull")
        (else
          (Variables|/Script/EasyBallistics.EBBarrel|SetShootingBlocked (Variables|Default|GetEBBarrel) true)
          (Variables|Default|SetbIsReloading true)
          (Animation|PlayAnimMontage (Variables|Default|GetWeaponOwner) (Variables|Default|GetPlayerReloadAnimMontage) 1.0 "None")
          (Audio|Components|Audio|Play (Variables|Default|GetReloadSound) 0.0)))
      (else
        (Development|PrintString "NoAmmoToReload")))))

(fn EndReload
  (bind _ebbarrel (Variables|Default|GetEBBarrel))
  (bind _ebbarrel_2 (Variables|Default|GetEBBarrel))
  (if (< (Variables|Default|GetRequiredAmmoCount) (Variables|Default|GetCurrentRemainingAmmo))
    (Variables|Default|SetCurrentRemainingAmmo (- (Variables|Default|GetCurrentRemainingAmmo) (Variables|Default|GetRequiredAmmoCount)))
    (Class|EBBarrel|SetAmmo _ebbarrel_2 (+ (Class|EBBarrel|GetAmmoCount (Variables|Default|GetEBBarrel) true) (Variables|Default|GetRequiredAmmoCount)) true false false (Class|EBBarrel|GetAmmo _ebbarrel_2 true))
    (else
      (Class|EBBarrel|SetAmmo _ebbarrel (+ (Class|EBBarrel|GetAmmoCount _ebbarrel true) (Variables|Default|GetCurrentRemainingAmmo)) false false false (Class|EBBarrel|GetAmmo _ebbarrel true))
      (Variables|Default|SetCurrentRemainingAmmo 0)))
  (Variables|/Script/EasyBallistics.EBBarrel|SetShootingBlocked (Variables|Default|GetEBBarrel) false)
  (Variables|Default|SetbIsReloading false)
  (Development|PrintString "ReloadingFinished"))

(fn GetCurrentRemainingAmmo
  (return (Variables|Default|GetCurrentRemainingAmmo)))

(fn GetCurrentMagazineAmmo
  (return (Class|EBBarrel|GetAmmoCount (Variables|Default|GetEBBarrel) true)))
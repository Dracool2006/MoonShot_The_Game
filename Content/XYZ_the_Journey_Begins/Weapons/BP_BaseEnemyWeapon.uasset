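; Base weapon Blueprint for AI enemies that aims its barrel at the owner's current target.
; The UpdateBarrelLocation event calls the parent, then draws a debug arrow from the barrel to its scaled forward vector, with no location offset added.
; If the owner is a BP_AI_BaseEnemy with a valid controller TargetEnemy, the barrel snaps to a look-at rotation toward that target.
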(event EventUpdateBarrelLocation
  (bind _ebbarrel (Variables|Default|GetEBBarrel))
  (|CallParentFunction)
  (Rendering|Debug|DrawDebugArrow (Transformation|GetWorldLocation _ebbarrel) (* (Math|Vector|GetForwardVector _ebbarrel) 100) 0.0 "(R=0.531250,G=0.032585,B=0.022015,A=1.000000)" 2.0 1.0)
  (bind _asbp_ai_base_enemy (Utilities|Casting|CastToBP_AI_BaseEnemy (Variables|Default|GetWeaponOwner)))
  (Utilities|IsValid (Variables|/Game/XYZ_the_Journey_Begins/Characters/AI/BaseEnemy/AIC_BaseEnemy.AIC_BaseEnemy_C|GetTargetEnemy (Variables|/Game/XYZ_the_Journey_Begins/Characters/AI/BaseEnemy/BP_AI_BaseEnemy.BP_AI_BaseEnemy_C|GetcontrollerRef _asbp_ai_base_enemy))
    (:Is%20Valid
      (Transformation|SetWorldRotation (Variables|Default|GetEBBarrel) (Math|Rotator|FindLookatRotation (Transformation|GetWorldLocation (Variables|Default|GetEBBarrel)) (Transformation|GetActorLocation (Variables|/Game/XYZ_the_Journey_Begins/Characters/AI/BaseEnemy/AIC_BaseEnemy.AIC_BaseEnemy_C|GetTargetEnemy (Variables|/Game/XYZ_the_Journey_Begins/Characters/AI/BaseEnemy/BP_AI_BaseEnemy.BP_AI_BaseEnemy_C|GetcontrollerRef _asbp_ai_base_enemy)))) false false))))

(fn ConstructionScript
  (|CallParentFunction))
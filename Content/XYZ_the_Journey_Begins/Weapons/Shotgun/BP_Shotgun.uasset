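; BP_Shotgun is the shotgun weapon Blueprint, supplying the cosmetic feedback for firing.
; Separate shoot events play and stop the fire animation on the weapon skeletal mesh, play a 2D fire sound on fire end, and attach a muzzle flash emitter to the MuzzleFlash socket.
; It holds no firing logic itself, and its construction script only calls the parent.
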(event EventPlayShootAnimation
  (params (bShootIsLoop :type Boolean))
  (Components|Animation|PlayAnimation (Variables|Default|GetWeapon_SkeletalMesh) "/Game/XYZ_the_Journey_Begins/Weapons/Shotgun/Anims/AS_Fire_Shotgun_W.AS_Fire_Shotgun_W" false))

(event EventShootSpawnMuzzleFlash
  (Effects|SpawnEmitterAttached "/Game/XYZ_the_Journey_Begins/Weapons/Shotgun/FX/P_Shotgun_MuzzleFlash.P_Shotgun_MuzzleFlash" (Variables|Default|GetWeapon_SkeletalMesh) "MuzzleFlash"))

(event EventStopShootAnimation
  (Audio|Components|Audio|Stop (Variables|Default|GetWeapon_SkeletalMesh)))

(event EventShootonFireEnd
  (Audio|PlaySound2D "/Game/XYZ_the_Journey_Begins/Weapons/Shotgun/Sound/Shotgun/Shotgun_Fire_Cue.Shotgun_Fire_Cue" 1.0 1.0 0.0 0 0))

(fn ConstructionScript
  (|CallParentFunction))
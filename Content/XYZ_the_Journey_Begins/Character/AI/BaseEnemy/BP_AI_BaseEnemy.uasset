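; BP_AI_BaseEnemy is the base enemy AI character, carrying a weapon through a child actor component.
; On BeginPlay it caches its AIC_BaseEnemy controller, then casts the child actor to BP_WeaponBase, stores it as the current weapon and sets itself as that weapon's owner.
; On death it runs the parent death logic, then tells the current weapon to stop shooting.
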(event EventBeginPlay
  (Utilities|FlowControl|Sequence
    (:then_0
      ;[1 1 1] Set AI Controller Ref
      (bind _asaic_base_enemy (Utilities|Casting|CastToAIC_BaseEnemy (Pawn|GetController)))
      (Variables|Pawn|SetcontrollerRef _asaic_base_enemy))
    (:then_1
      (bind _asbp_weapon_base (Utilities|Casting|CastToBP_WeaponBase (Variables|/Script/Engine.ChildActorComponent|GetChildActor (Variables|Default|GetWeaponActor))))
      (bind _output_get (Variables|Weapon|SetCurrentWeapon _asbp_weapon_base))
      (Variables|/Game/XYZ_the_Journey_Begins/Weapons/BP_WeaponBase.BP_WeaponBase_C|SetWeaponOwner _output_get self))))

(event EventOnDeath
  (|CallParentFunction)
  (Default|StopShoot (Variables|Weapon|GetCurrentWeapon)))

(fn ConstructionScript)
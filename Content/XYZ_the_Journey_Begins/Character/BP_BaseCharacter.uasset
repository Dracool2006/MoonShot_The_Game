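; Base character Blueprint that provides shared health and death handling.
; Any damage reduces CurrentHealth, clamped between zero and MaxHealth, and triggers OnDeath with a debug "IM DEAD" print when health runs out.
; OnDeath sets IsDead, calls the OnDead dispatcher and plays DeathMontage on the mesh.
; GetHealth returns current health as a normalized fraction of the maximum.
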(event Custom|OnDeath
  (bind _mesh (Variables|Character|GetMesh))
  ;[1 1 1] Event onDeath
  (Variables|DeathSystem|SetbIsDead true)
  (Default|CallOnDead)
  (Utilities|IsValid _mesh
    (:Is%20Valid
      (Animation|Montage|PlayMontage _mesh (Variables|DeathSystem|GetDeathMontage)))))

(event Game|Damage|EventAnyDamage
  (params (Damage :type Float%20%28single-precision%29) (DamageType :type Damage%20Type%20Object%20Reference) (InstigatedBy :type Controller%20Object%20Reference) (DamageCauser :type Actor%20Object%20Reference))
  ;[1 1 1] Change HP on Any Damage
  (if (> (Variables|HealthSystem|GetCurrentHealth) 0.0)
    (bind _output_get (Variables|HealthSystem|SetCurrentHealth (Math|Float|Clamp(Float) (- (Variables|HealthSystem|GetCurrentHealth) Damage) 0.0 (Variables|HealthSystem|GetMaxHealth))))
    (if (<= _output_get 0.0)
      (Development|PrintString "IM DEAD" true true "(R=0.234375,G=0.021468,B=0.035467,A=1.000000)" 3.0)
      (CallFunction|OnDeath))))

(fn ConstructionScript)

(fn GetHealth
  (return (Math|Float|Clamp(Float) (/ (Variables|HealthSystem|GetCurrentHealth) (Variables|HealthSystem|GetMaxHealth)))))
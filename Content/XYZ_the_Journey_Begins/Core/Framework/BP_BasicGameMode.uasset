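; Game mode that declares a win once every enemy in its EnemiesToKill list has died.
; On BeginPlay it binds a handler to the post-death event of each valid entry in that list.
; Each death increments KillCount, and OnWin is called when the count equals the list length.
; Invalid entries are skipped when binding but still count toward that total.
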(event Custom|Event%20OnPostDead
  (bind _result (Math|Integer|IncrementInt (Variables|Default|GetkillCount))
    (:%20%20
      (Variables|Default|SetkillCount _result)
      (if (== (Utilities|Array|Length (Variables|Default|GetEnemiesToKill)) (Variables|Default|GetkillCount))
        (Default|CallOnWin)))))

(event EventBeginPlay
  (for _array_element (Variables|Default|GetEnemiesToKill)
    (Utilities|IsValid (Utilities|ResolveSoftReference _array_element)
      (:Is%20Valid
        (EventDispatchers|BindEventtoOnPostDead (Utilities|ResolveSoftReference _array_element) (delegate Custom|Event%20OnPostDead))))))

(fn ConstructionScript)